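; BP_Lock is a clickable combination lock with four rotating rings.
; Clicking a ring while the lock is not unlocked turns it 36 degrees from its current relative rotation, giving ten positions per turn.
; Each turn then calls CheckRotation, whose logic is not shown here, and the Unlock flag blocks further turning once set.
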(event OnClicked(Ring1)
  (params (TouchedComponent :type Primitive%20Component%20Object%20Reference) (ButtonPressed :type Key%20Structure :default "None"))
  (if (not (Variables|Default|GetbUnlock))
    (Transformation|SetRelativeRotation TouchedComponent (Math|Rotator|CombineRotators (Variables|/Script/Engine.SceneComponent|GetRelativeRotation TouchedComponent) (Math|Rotator|MakeRotator 36.0 0.0 0.0)) false false)
    (Class|Lock|CheckRotation)))

(event OnClicked(Ring2)
  (params (TouchedComponent :type Primitive%20Component%20Object%20Reference) (ButtonPressed :type Key%20Structure :default "None"))
  (if (not (Variables|Default|GetbUnlock))
    (Transformation|SetRelativeRotation TouchedComponent (Math|Rotator|CombineRotators (Variables|/Script/Engine.SceneComponent|GetRelativeRotation TouchedComponent) "0.000000,0.000000,36.000000") false false)
    (Class|Lock|CheckRotation)))

(event OnClicked(Ring3)
  (params (TouchedComponent :type Primitive%20Component%20Object%20Reference) (ButtonPressed :type Key%20Structure :default "None"))
  (if (not (Variables|Default|GetbUnlock))
    (Transformation|SetRelativeRotation TouchedComponent (Math|Rotator|CombineRotators (Variables|/Script/Engine.SceneComponent|GetRelativeRotation TouchedComponent) "0.000000,0.000000,36.000000") false false)
    (Class|Lock|CheckRotation)))

(event OnClicked(Ring4)
  (params (TouchedComponent :type Primitive%20Component%20Object%20Reference) (ButtonPressed :type Key%20Structure :default "None"))
  (if (not (Variables|Default|GetbUnlock))
    (Transformation|SetRelativeRotation TouchedComponent (Math|Rotator|CombineRotators (Variables|/Script/Engine.SceneComponent|GetRelativeRotation TouchedComponent) "0.000000,0.000000,36.000000") false false)
    (Class|Lock|CheckRotation)))

(fn ConstructionScript)