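; BP_KidTrain is a train actor assembled procedurally in its construction script, with no active event graph logic.
; Once SetLocomotivePos succeeds, it adds a configurable number of wagon static mesh components, each offset along X by wagon size.
; SetNewWagonColor colors each wagon as it is created.
; The collected components are stored in Wagons, then UpdateWagonPos adjusts their placement.
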(event EventBeginPlay)

(event Collision|EventActorBeginOverlap
  (params (OtherActor :type Actor%20Object%20Reference)))

(event EventTick
  (params (DeltaSeconds :type Float%20%28single-precision%29)))

(fn ConstructionScript
  (bind _returnvalue (Class|Train|SetLocomotivePos))
  (if _returnvalue
    (for _index (range 0 (- (Variables|Default|GetNumberOfWagon) 1))
      (bind _returnvalue_2 (Class|Train|GetWagonSize))
      (bind _returnvalue_3 (AddComponent|AddStaticMeshComponent false (Math|Transform|MakeTransform (Math|Vector|MakeVector (+ _returnvalue_2 (* _returnvalue_2 _index)) 0.0 0.0) "0, 0, 0" "1.000000,1.000000,1.000000")))
      (Class|Train|SetNewWagonColor _returnvalue_3)
      (Utilities|Array|AddUnique (LocalVariables|GetListOfWagons) _returnvalue_3))
    (Variables|Default|SetWagons (LocalVariables|GetListOfWagons))
    (Class|Train|UpdateWagonPos)))