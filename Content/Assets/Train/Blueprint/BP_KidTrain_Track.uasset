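; Kid train track actor that lays spline meshes along its Spline component to form a continuous track.
; The construction script gets a segment length and index count, then adds a spline mesh component for each segment.
; Each segment takes local positions and tangents from the spline at its start and end distances, with tangents clamped to segment length to limit distortion.
; The event graph holds no runtime logic.
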(event EventBeginPlay)

(event Collision|EventActorBeginOverlap
  (params (OtherActor :type Actor%20Object%20Reference)))

(event EventTick
  (params (DeltaSeconds :type Float%20%28single-precision%29)))

(fn ConstructionScript
  (bind _returnvalue (Class|Track|GetXSize))
  (LocalVariables|SetxSize _returnvalue)
  (bind _returnvalue_2 (Class|Track|GetMaxIndex))
  (for _index (range 0 _returnvalue_2)
    (bind _returnvalue_3 (AddComponent|AddSplineMeshComponent false))
    (SplineMesh|SetStartandEnd _returnvalue_3 (Spline|GetLocationatDistanceAlongSpline (Variables|Default|GetSpline) (* _index (LocalVariables|GetxSize)) "Local") (Math|Vector|ClampVectorSize (Spline|GetTangentatDistanceAlongSpline (Variables|Default|GetSpline) (* _index (LocalVariables|GetxSize)) "Local") 0.0 (LocalVariables|GetxSize)) (Spline|GetLocationatDistanceAlongSpline (Variables|Default|GetSpline) (* (+ _index 1) (LocalVariables|GetxSize)) "Local") (Math|Vector|ClampVectorSize (Spline|GetTangentatDistanceAlongSpline (Variables|Default|GetSpline) (* (+ _index 1) (LocalVariables|GetxSize)) "Local") 0.0 (LocalVariables|GetxSize)) true :!class /Script/Engine.SplineMeshComponent)))

(fn GetNewMesh
  (bind _returnvalue (AddComponent|AddSplineMeshComponent false))
  (return _returnvalue))