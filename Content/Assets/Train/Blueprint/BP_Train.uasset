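; BP_Train is a train actor that builds its line of wagons in the Construction Script, with no active runtime logic.
; A loop over NumberOfWagons adds instances to yellow, blue, green and red wagon instanced mesh components, selected by an incrementing index that wraps at four.
; Each instance is offset along negative Y by an index-based multiple of a fixed spacing.
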(event EventBeginPlay)

(event Collision|EventActorBeginOverlap
  (params (OtherActor :type Actor%20Object%20Reference)))

(event EventTick
  (params (DeltaSeconds :type Float%20%28single-precision%29)))

(fn ConstructionScript
  (for _index (range 0 (- (Variables|Default|GetNumberOfWagons) 1))
    (bind _result (Math|Integer|IncrementInt (Variables|Default|GetIndex))
      (:%20%20
        (if (>= _result 4)
          (Variables|Default|SetIndex 0))
        (Components|InstancedStaticMesh|AddInstance (Utilities|Select :Index (Variables|Default|GetIndex) :Option%200 (Variables|Default|GetYellowWagon) :Option%201 (Variables|Default|GetBlueWagon) :Option%202 (Variables|Default|GetGreenWagon) :Option%203 (Variables|Default|GetRedWagon)) (Math|Transform|MakeTransform (Math|Vector|MakeVector 0.0 (Math|Conversions|ToFloat(Integer) (* (+ _index 1) -30)) 0.0) "0, 0, 0" "1.000000,1.000000,1.000000") false)))))